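; BP_DialogueHandler pushes dialogue subtitles (speaker name and body text) to the main HUD when play begins.
; GetCurrentLine reads FDialogue, taking body text from the map's keys at CurrentDialogueSequenceIndex.
; BeginPlay shows the current line, waits a fixed delay, then advances the index and shows one more line.
; TriggerTime is looked up by the index as a name rather than the line's key, and BeginPlay never uses it.
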(event `self.ReceiveBeginPlay`
  (bind (_speakername _bodytext) (`self.GetCurrentLine`))
  (bind (_speakername_2 _bodytext_2) (`self.GetCurrentLine`))
  (`/Game/OptionsSystem/HUD/BP_GameHUD.UpdateSubtitles` (`/Game/OptionsSystem/HUD/BPFL_HUD.BPFL_GetMainHUD`) (`KismetTextLibrary.Conv_NameToText` _speakername_2) (`KismetTextLibrary.Conv_NameToText` _bodytext_2))
  (`KismetSystemLibrary.Delay` 4.0)
  (`/Engine/EditorBlueprintResources/StandardMacros.IncrementInt` (`self.CurrentDialogueSequenceIndex`)
    (:`  `
      (`/Game/OptionsSystem/HUD/BP_GameHUD.UpdateSubtitles` (`/Game/OptionsSystem/HUD/BPFL_HUD.BPFL_GetMainHUD`) (`KismetTextLibrary.Conv_NameToText` _speakername) (`KismetTextLibrary.Conv_NameToText` _bodytext)))))

(fn `GetCurrentLine`
  (returns (SpeakerName :type Name) (BodyText :type Name) (TriggerTime :type "Float (double-precision)"))
  (locals (Local_BodyText :type "Map of Name to Float (double-precision)"))
  (bind (_speakername _bodytext) (break `/Game/OptionsSystem/HUD/Subtitles/F_Dialogue` (`self.F_Dialogue`)))
  (bind _keys (`BlueprintMapLibrary.Map_Keys` _bodytext))
  (return _speakername (`|GetArrayItem` _keys (`self.CurrentDialogueSequenceIndex`)) (`BlueprintMapLibrary.Map_Find` _bodytext (`KismetStringLibrary.Conv_StringToName` (`KismetStringLibrary.Conv_IntToString` (`self.CurrentDialogueSequenceIndex`))))))

(fn `UserConstructionScript`)